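; Pressure-plate code puzzle actor that opens a linked Door when the player steps on plates in the right sequence.
; The construction script builds a row of plates sized to Correctcode, each with an overlap box tagged by a RandomCode character.
; Player overlaps play click sounds and prepend unused characters to InputCode, so Correctcode matches in reverse press order.
; At full length, a match opens the door; a mismatch clears the input.
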(fn `AddCode`
  (params (Add :type String))
  (set `self.InputCode` (`KismetStringLibrary.Concat_StrStr` Add (`self.InputCode`)))
  (if (== (`KismetStringLibrary.Len` (`self.correctcode`)) (`KismetStringLibrary.Len` (`self.InputCode`)))
    (if (== (`self.correctcode`) (`self.InputCode`))
      (`/Game/Blueprints/BP_door.Open Door` (`self.Door`))
      (else
        (`KismetSystemLibrary.PrintString` "incorect code")
        (set `self.InputCode` "")))
    (else
      (`KismetSystemLibrary.PrintString` "invalid length"))))

(fn `BP_pressPuzzle_AutoGenFunc`
  (params (OverlappedComponent :type "PrimitiveComponent Object Reference") (OtherActor :type "Actor Object Reference") (OtherComp :type "PrimitiveComponent Object Reference") (OtherBodyIndex :type Integer) (bFromSweep :type Boolean) (SweepResult :type "HitResult Structure (by ref)"))
  (bind _returnvalue (`KismetStringLibrary.Conv_NameToString` (`|GetArrayItem` (`ActorComponent.ComponentTags` OverlappedComponent))))
  (cast `/Game/FirstPerson/Blueprints/BP_FirstPersonCharacter` OtherActor)
  (if (`KismetStringLibrary.Contains` (`self.InputCode`) _returnvalue)
    (`GameplayStatics.PlaySoundAtLocation` "/Game/SoundEffects/43688__stijn__click8b.43688__stijn__click8b" (0.0 0.0 0.0) (struct) 1.0 1.0 0.0 null null null null)
    (else
      (`GameplayStatics.PlaySoundAtLocation` "/Game/SoundEffects/113636__edgardedition__click6.113636__edgardedition__click6" (0.0 0.0 0.0) (struct) 1.0 1.0 0.0 null null null null)
      (`self.AddCode` _returnvalue)
      (return))))

(fn `UserConstructionScript`
  (for _index (range (`KismetStringLibrary.Len` (`self.correctcode`)))
    (bind _returnvalue (`AddComponent|NODE_AddStaticMeshComponent-0` :`RelativeTransform` (`KismetMathLibrary.MakeTransform` (`KismetMathLibrary.MakeVector` (* _index (`self.spacing`))) (struct) (0.4 0.4 0.1))))
    (`PrimitiveComponent.SetMaterial` _returnvalue 0 "/Game/materials/M_DamagedMetal.M_DamagedMetal")
    (bind _returnvalue_2 (`AddComponent|NODE_AddBoxComponent-0` :`RelativeTransform` (`KismetMathLibrary.MakeTransform` (+ (`SceneComponent.RelativeLocation` _returnvalue) (0.0 0.0 50.0)))))
    (set `ActorComponent.ComponentTags` (`|MakeArray` (`KismetStringLibrary.Conv_StringToName` (`KismetStringLibrary.GetSubstring` (`self.RandomCode`) _index))) _returnvalue_2)
    (add `PrimitiveComponent.OnComponentBeginOverlap` _returnvalue_2 (`|CreateDelegate` :!event `BP_pressPuzzle_AutoGenFunc`))))