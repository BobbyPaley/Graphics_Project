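; BP_gun is a gun pickup actor that shows a widget while something overlaps its Box component.
; Its construction script sets the Firelock mesh from the ItemModelToPickUp variable.
; The PickUp event only prints an acquired message and destroys the actor after a short delay, with no weapon granted here.
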(event `/Game/Blueprints/BPI_guns.PickUp`
  (`KismetSystemLibrary.PrintString` "Gun aquired")
  (`KismetSystemLibrary.Delay` 1.0)
  (`self.K2_DestroyActor`))

(event `self.Box.OnComponentBeginOverlap`
  (params (OverlappedComponent :type "PrimitiveComponent Object Reference") (OtherActor :type "Actor Object Reference") (OtherComp :type "PrimitiveComponent Object Reference") (OtherBodyIndex :type Integer) (bFromSweep :type Boolean) (SweepResult :type "HitResult Structure (by ref)"))
  (`SceneComponent.SetVisibility` (`self.Widget`) true false))

(event `self.Box.OnComponentEndOverlap`
  (params (OverlappedComponent :type "PrimitiveComponent Object Reference") (OtherActor :type "Actor Object Reference") (OtherComp :type "PrimitiveComponent Object Reference") (OtherBodyIndex :type Integer))
  (`SceneComponent.SetVisibility` (`self.Widget`) false false))

(fn `UserConstructionScript`
  (`StaticMeshComponent.SetStaticMesh` (`self.firelock`) (`self.ItemModelToPickUp`)))