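; Stun grenade projectile that either stuns an enemy on impact or sticks to a wall to open a hole.
; On hit, it attaches to unoccupied Stickable BP_wall actors, explodes on unstunned BP_Enemy targets, and self-destroys on other surfaces.
; Explode, not called within this Blueprint, spawns a BP_HoleZone using the stored wall and hit data.
; It registers with the player character on BeginPlay and unregisters on EndPlay unless a hole was created.
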(event `self.ReceiveEndPlay`
  (params (EndPlayReason :type "EEndPlayReason Enum" :default "Destroyed"))
  ; Unregistering projectile
  (if (not (`self.validHole?`))
    (bind _asbp_first_person_character (cast `/Game/FirstPerson/Blueprints/BP_FirstPersonCharacter` (`GameplayStatics.GetPlayerCharacter` 0)))
    (`/Game/FirstPerson/Blueprints/BP_FirstPersonCharacter.UnregisterProjectile` _asbp_first_person_character)
    (`KismetSystemLibrary.PrintString` "Unregistered")))

(event `self.ReceiveBeginPlay`
  ; Register projectile
  (bind _asbp_first_person_character (cast `/Game/FirstPerson/Blueprints/BP_FirstPersonCharacter` (`GameplayStatics.GetPlayerCharacter` 0)))
  (`/Game/FirstPerson/Blueprints/BP_FirstPersonCharacter.RegisterProjectile` _asbp_first_person_character))

(event `self.ReceiveHit`
  (params (MyComp :type "PrimitiveComponent Object Reference") (Other :type "Actor Object Reference") (OtherComp :type "PrimitiveComponent Object Reference") (bSelfMoved :type Boolean) (HitLocation :type "Vector Structure") (HitNormal :type "Vector Structure") (NormalImpulse :type "Vector Structure") (Hit :type "HitResult Structure (by ref)"))
  (set `self.Hit Location` HitLocation)
  (set `self.HitNormal` HitNormal)
  (`KismetSystemLibrary.PrintString` "hit detected")
  (if (`self.ActorHasTag` Other "Stickable")
    (bind _asbp_wall (cast `/Game/Blueprints/BP_wall` Other))
    (if (`/Game/Blueprints/BP_wall.stuck` _asbp_wall)
      (`KismetSystemLibrary.PrintString` "already stuck")
      (`self.K2_DestroyActor`)
      (else
        (`MovementComponent.StopMovementImmediately` (`self.ProjectileMovement`))
        (set `ProjectileMovementComponent.ProjectileGravityScale` 0.0 (`self.ProjectileMovement`))
        (`PrimitiveComponent.SetCollisionEnabled` (`self.stun_grenade`) "NoCollision")
        (`PrimitiveComponent.SetCollisionEnabled` (`self.Sphere`) "NoCollision")
        (`self.K2_SetActorLocation` (+ HitLocation (* HitNormal (`self.5`))))
        (`self.K2_SetActorRotation` (`KismetMathLibrary.MakeRotFromX` HitNormal))
        (`self.K2_AttachToComponent` OtherComp "None" "KeepWorld" "KeepWorld" "KeepWorld")
        (set `self.stuckOnWall` true)
        (bind _asbp_wall_2 (cast `/Game/Blueprints/BP_wall` Other))
        (set `self.wall` _asbp_wall_2)
        (set `/Game/Blueprints/BP_wall.stuck` true _asbp_wall_2)))
    (else
      (bind _asbp_enemy (cast `/Game/Blueprints/Enemy/BP_Enemy` Other)
        (:`then`
          (if (`/Game/Blueprints/Enemy/BP_Enemy.stunned?` _asbp_enemy)
            (`KismetSystemLibrary.PrintString` "already stunned")
            (else
              (`KismetSystemLibrary.PrintString` "actor is enemy")
              (set `/Game/Blueprints/Enemy/BP_Enemy.stunned?` true _asbp_enemy)
              (`GameplayStatics.PlaySoundAtLocation` "/Game/SoundEffects/341626__aceofspadesproduc100__small-boom.341626__aceofspadesproduc100__small-boom" (`SceneComponent.K2_GetComponentLocation` (`Character.Mesh` _asbp_enemy)) (struct) 1.0 1.0 0.0 null null null null)
              (`NiagaraFunctionLibrary.SpawnSystemAtLocation` "/Game/VFX/ns_explosion.ns_explosion" (`self.Hit Location`))
              (`self.K2_DestroyActor`))))
        (:`CastFailed`
          (`KismetSystemLibrary.PrintString` "inavlid wall")
          (`self.K2_DestroyActor`))))))

(fn `Explode`
  (bind _hit_location (`self.Hit Location`))
  ; delete later
  (bind _asbp_first_person_character (cast `/Game/FirstPerson/Blueprints/BP_FirstPersonCharacter` (`GameplayStatics.GetPlayerCharacter` 0)))
  (`|SpawnActorFromClass` "/Game/Blueprints/BP_HoleZone.BP_HoleZone_C" (`self.GetTransform`) "Undefined" "MultiplyWithRoot" null (`self.wall`) 200.0 _asbp_first_person_character _hit_location (`self.HitNormal`) null)
  (`GameplayStatics.PlaySoundAtLocation` "/Game/SoundEffects/341626__aceofspadesproduc100__small-boom.341626__aceofspadesproduc100__small-boom" _hit_location (struct) 1.0 1.0 0.0 null null null null)
  (`NiagaraFunctionLibrary.SpawnSystemAtLocation` "/Game/VFX/ns_explosion.ns_explosion" _hit_location)
  (`KismetSystemLibrary.PrintString` "Spawning hole zone")
  (set `self.validHole?` true)
  (`self.K2_DestroyActor`))

(fn `UserConstructionScript`)