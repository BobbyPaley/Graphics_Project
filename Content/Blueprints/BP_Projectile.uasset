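; Sticky stun grenade projectile that clings to surfaces of actors tagged Stickable and destroys itself on hitting anything else.
; On a Stickable hit it halts projectile movement, zeroes gravity and disables grenade collision.
; It then offsets itself along the hit normal, aligns to that normal, attaches to the hit component keeping world transform, and flags itself Stuck.
; No stun effect is implemented here; debug prints report hits and destruction.
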(event `self.ReceiveHit`
  (params (MyComp :type "PrimitiveComponent Object Reference") (Other :type "Actor Object Reference") (OtherComp :type "PrimitiveComponent Object Reference") (bSelfMoved :type Boolean) (HitLocation :type "Vector Structure") (HitNormal :type "Vector Structure") (NormalImpulse :type "Vector Structure") (Hit :type "HitResult Structure (by ref)"))
  (`KismetSystemLibrary.PrintString` "hit detected")
  (if (`self.ActorHasTag` Other "Stickable")
    (`MovementComponent.StopMovementImmediately` (`self.ProjectileMovement`))
    (set `ProjectileMovementComponent.ProjectileGravityScale` 0.0 (`self.ProjectileMovement`))
    (`PrimitiveComponent.SetCollisionEnabled` (`self.stun_grenade`) "NoCollision")
    (`self.K2_SetActorLocation` (+ HitLocation (* HitNormal (`self.5`))))
    (`self.K2_SetActorRotation` (`KismetMathLibrary.MakeRotFromX` HitNormal))
    (`self.K2_AttachToComponent` OtherComp "None" "KeepWorld" "KeepWorld" "KeepWorld")
    (set `self.stuck` true)
    (else
      (`KismetSystemLibrary.PrintString` "actor destroyed")
      (`self.K2_DestroyActor`))))

(fn `UserConstructionScript`)