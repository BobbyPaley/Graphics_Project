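; BP_Enemy is a melee enemy that chases the player on sight and punches at close range, with a short attack cooldown.
; PawnSensing triggers an AI MoveTo toward the player, then a punch montage, while EnemyAttackHit applies damage and plays an impact sound.
; When hit while Stunned, it disables movement and physical collision, plays death and reversed-death montages to fall and rise, then restores itself.
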(event `self.PawnSensing.OnSeePawn`
  (params (Pawn :type "Pawn Object Reference"))
  (if (not (`self.stunned?`))
    (set `self.isSeeingPlayer?` true)
    (`self.FollowPlayer`)))

(event `FollowPlayer`
  (if (`self.stunned?`)
    (`KismetSystemLibrary.PrintString` "stunned")
    (else
      (set `self.canAttack?` true)
      (if (`self.isSeeingPlayer?`)
        (`|AIMoveTo` self (0.0 0.0 0.0) (`GameplayStatics.GetPlayerCharacter` 0)
          (:`OnSuccess`
            (if (`self.canAttack?`)
              (if (<= (`KismetMathLibrary.Vector_Distance` (`self.K2_GetActorLocation` (`GameplayStatics.GetPlayerCharacter` 0)) (`self.K2_GetActorLocation`)) 150.0)
                (set `self.canAttack?` false)
                (`self.PlayAnimMontage` "/Game/Characters/Swat/Animations/AL_punch_montage.AL_punch_montage" 1.5)
                (`KismetSystemLibrary.Delay` 2.0)
                (set `self.canAttack?` true)))))))))

(event `self.ReceiveHit`
  (params (MyComp :type "PrimitiveComponent Object Reference") (Other :type "Actor Object Reference") (OtherComp :type "PrimitiveComponent Object Reference") (bSelfMoved :type Boolean) (HitLocation :type "Vector Structure") (HitNormal :type "Vector Structure") (NormalImpulse :type "Vector Structure") (Hit :type "HitResult Structure (by ref)"))
  (`KismetSystemLibrary.Delay` 0.02)
  (if (`self.stunned?`)
    (if (== (`self.hitNumber`) 0)
      (`CharacterMovementComponent.DisableMovement` (`self.CharacterMovement`))
      (set `self.hitNumber` 1)
      (`PrimitiveComponent.SetCollisionEnabled` (`self.CapsuleComponent`) "QueryOnly")
      (set `self.bUseControllerRotationYaw` false)
      (set `CharacterMovementComponent.bOrientRotationToMovement` false (`self.CharacterMovement`))
      (bind _returnvalue (`self.PlayAnimMontage` "/Game/Characters/Swat/Animations/AL_Swat_Anim_Rig_Death01_Montage.AL_Swat_Anim_Rig_Death01_Montage"))
      (`KismetSystemLibrary.Delay` (- _returnvalue 0.3))
      (`KismetSystemLibrary.PrintString` "anim 1 finish")
      (bind _returnvalue_2 (`self.PlayAnimMontage` "/Game/Characters/Swat/Animations/Al_standard_death_reverse_Montage.Al_standard_death_reverse_Montage"))
      (`KismetSystemLibrary.Delay` (- _returnvalue_2 0.3))
      (set `self.stunned?` false)
      (`CharacterMovementComponent.SetMovementMode` (`self.CharacterMovement`) "MOVE_Walking" 0)
      (set `self.bUseControllerRotationYaw` true)
      (set `CharacterMovementComponent.bOrientRotationToMovement` true (`self.CharacterMovement`))
      (`PrimitiveComponent.SetCollisionEnabled` (`self.CapsuleComponent`) "QueryAndPhysics")
      (set `self.hitNumber` 0))))

(fn `EnemyAttackHit`
  (bind _asbp_first_person_character (cast `/Game/FirstPerson/Blueprints/BP_FirstPersonCharacter` (`GameplayStatics.GetPlayerCharacter` 0)))
  (`/Game/FirstPerson/Blueprints/BP_FirstPersonCharacter.TakeDamage` _asbp_first_person_character 20.0)
  (`KismetSystemLibrary.PrintString` "Hit")
  (`GameplayStatics.PlaySoundAtLocation` "/Game/SoundEffects/classic-punch-impact-352711.classic-punch-impact-352711" (`SceneComponent.K2_GetComponentLocation` (`self.CapsuleComponent`)) (struct) 1.0 1.0 0.0 null null null null))

(fn `UserConstructionScript`)