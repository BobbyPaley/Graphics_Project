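; Pressure switch actor for a button puzzle that signals a linked door while something overlaps it.
; Begin overlap calls SwitchActivated on DoorToActivate, sets Active, prints a debug message and plays the SwitchActivate timeline, which drives the Switch component's relative Z.
; End overlap calls SwitchDeactivated, clears Active and reverses the timeline.
; Overlaps are neither filtered nor counted, so any single exit deactivates the switch.
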(event `self.ReceiveActorBeginOverlap`
  (params (OtherActor :type "Actor Object Reference"))
  (`/Game/Blueprints/Button_Puzzle/BP_Door.SwitchActivated` (`self.doorToActivate`))
  (`KismetSystemLibrary.PrintString` "switch activated called")
  (set `self.Active?` true)
  (bind (_direction _switchposition) (`Timeline|SwitchActivate` :!label _label)
    (:`Update`
      (`SceneComponent.K2_SetRelativeLocation` (`self.Switch`) (`KismetMathLibrary.MakeVector` 0.0 0.0 _switchposition) false false))))

(event `self.ReceiveActorEndOverlap`
  (params (OtherActor :type "Actor Object Reference"))
  (`/Game/Blueprints/Button_Puzzle/BP_Door.SwitchDeactivated` (`self.doorToActivate`))
  (set `self.Active?` false)
  (goto _label :!via `Reverse`))

(fn `UserConstructionScript`)