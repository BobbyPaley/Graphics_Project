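; BP_Door is a puzzle door that opens once enough pressure switches are active at the same time.
; SwitchActivated and SwitchDeactivated raise and lower an active-switch count, and reaching the required count plays the DoorActivation timeline.
; The timeline drives the Door component's relative Z location.
; Any switch deactivation reverses the timeline, without rechecking the count.
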(event `SwitchActivated`
  (bind _pressureswitchesactive (`self.PressureSwitchesActive`))
  (`/Engine/EditorBlueprintResources/StandardMacros.IncrementInt` _pressureswitchesactive
    (:`  `
      (if (>= _pressureswitchesactive (`self.PressureSwitchesNeeded`))
        (bind (_direction _door_position) (`Timeline|DoorActivation` :!label _label)
          (:`Update`
            (`SceneComponent.K2_SetRelativeLocation` (`self.Door`) (`KismetMathLibrary.MakeVector` 0.0 0.0 _door_position) false false)))))))

(event `SwitchDeactivated`
  (`/Engine/EditorBlueprintResources/StandardMacros.DecrementInt` (`self.PressureSwitchesActive`)
    (:`  `
      (goto _label :!via `Reverse`))))

(fn `UserConstructionScript`)