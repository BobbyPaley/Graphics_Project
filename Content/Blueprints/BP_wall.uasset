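; BP_wall is a wall Blueprint whose material takes a positioned hole of variable radius.
; On BeginPlay it creates a dynamic instance of M_PassingWall on its Cube and stores it as MIDWall.
; UpdateHole writes a given center and radius to that instance's HoleCenter3D and HoleRadius parameters, leaving the hole effect to the material.
; The radius check at the end of UpdateHole has no effect.
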(event `self.ReceiveBeginPlay`
  (bind _returnvalue (`PrimitiveComponent.CreateDynamicMaterialInstance` (`self.Cube`) 0 "/Game/materials/M_PassingWall.M_PassingWall" "None"))
  (`PrimitiveComponent.SetMaterial` (`self.Cube`) 0 _returnvalue)
  (set `self.MID_wall` _returnvalue))

(fn `UpdateHole`
  (params (HoleCenter :type "Vector Structure") (HoleRadius :type "Float (double-precision)"))
  (bind _mid_wall (`self.MID_wall`))
  (`MaterialInstanceDynamic.SetVectorParameterValue` _mid_wall "HoleCenter3D" (`KismetMathLibrary.Conv_VectorToLinearColor` HoleCenter))
  (`MaterialInstanceDynamic.SetScalarParameterValue` _mid_wall "HoleRadius" HoleRadius)
  (if (> HoleRadius 0.0)
    _))

(fn `UserConstructionScript`)