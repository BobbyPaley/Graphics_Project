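; Temporary hole zone on a target wall that lets the player, enemies and crates pass through while it shrinks.
; A timeline shrinks the sphere and updates the wall's hole, then destroys the actor and clears the wall's Stuck flag.
; Overlaps toggle move-ignore for characters and wall channel responses for camera and crates.
; TryTransfer offers velocity-checked teleporting across the wall but is never called here.
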(event `self.ReceiveEndPlay`
  (params (EndPlayReason :type "EEndPlayReason Enum" :default "Destroyed"))
  (`/Game/FirstPerson/Blueprints/BP_FirstPersonCharacter.UnregisterProjectile` (`self.PlayerRef`)))

(event `self.ReceiveBeginPlay`
  (bind _currentradius (`self.CurrentRadius`))
  (`KismetSystemLibrary.Delay` 0.02)
  (`/Engine/EditorBlueprintResources/StandardMacros.IsValid` (`self.TargetWall`)
    (:`Is Valid`
      (bind _output_get (set `self.HoleNormal` (`KismetMathLibrary.Normal` (`self.HoleNormal`))))
      (set `self.CurrentRadius` (`self.InitialRadius`))
      (bind _returnvalue (* _output_get (+ 10.0 (* 0.5 (`self.wallThicknessGuess`)))))
      (`SceneComponent.K2_SetWorldLocation` (`self.FrontTrigger`) (+ _returnvalue (`self.HoleCenter`)) false false)
      (`SceneComponent.K2_SetWorldLocation` (`self.BackTrigger`) (- (`self.HoleCenter`) _returnvalue) false false)
      (bind (_direction _shrinkalpha) (`Timeline|Shrink` :!via `PlayFromStart`)
        (:`Update`
          (set `self.CurrentRadius` (`KismetMathLibrary.Lerp` (`self.InitialRadius`) 0.0 _shrinkalpha))
          (`SphereComponent.SetSphereRadius` (`self.Sphere`) _currentradius true)
          (`/Game/Blueprints/BP_wall.UpdateHole` (`self.TargetWall`) (`SceneComponent.K2_GetComponentLocation` (`self.Sphere`)) _currentradius))
        (:`Finished`
          (`self.K2_DestroyActor`)
          (`KismetSystemLibrary.PrintString` "Hole zone destroyed")
          (set `/Game/Blueprints/BP_wall.stuck` false (`self.TargetWall`)))))
    (:`Is Not Valid`
      (`self.K2_DestroyActor`)
      (`KismetSystemLibrary.PrintString` "invalid bp wall reference passed to hole Zone"))))

(event `self.Sphere.OnComponentBeginOverlap`
  (params (OverlappedComponent :type "PrimitiveComponent Object Reference") (OtherActor :type "Actor Object Reference") (OtherComp :type "PrimitiveComponent Object Reference") (OtherBodyIndex :type Integer) (bFromSweep :type Boolean) (SweepResult :type "HitResult Structure (by ref)"))
  (bind _targetwall (`self.TargetWall`))
  (bind _targetwall_2 (`self.TargetWall`))
  (bind _asbp_first_person_character (cast `/Game/FirstPerson/Blueprints/BP_FirstPersonCharacter` OtherActor)
    (:`then`
      (bind _capsulecomponent (`Character.CapsuleComponent` _asbp_first_person_character))
      (`/Engine/EditorBlueprintResources/StandardMacros.IsValid` _capsulecomponent
        (:`Is Valid`
          (set `self.playerCapsuleRadius` (`CapsuleComponent.GetScaledCapsuleRadius` _capsulecomponent))
          (`PrimitiveComponent.IgnoreActorWhenMoving` (`MovementComponent.UpdatedPrimitive` (`Character.CharacterMovement` _asbp_first_person_character)) _targetwall_2 true)
          (`PrimitiveComponent.SetCollisionResponseToChannel` (`/Game/Blueprints/BP_wall.Cube` _targetwall_2) "ECC_Camera" "ECR_Ignore"))
        (:`Is Not Valid`
          (`KismetSystemLibrary.PrintString` "un able to detect capsule"))))
    (:`CastFailed`
      (bind _asbp_enemy (cast `/Game/Blueprints/Enemy/BP_Enemy` OtherActor)
        (:`then`
          (bind _capsulecomponent_2 (`Character.CapsuleComponent` _asbp_enemy))
          (`/Engine/EditorBlueprintResources/StandardMacros.IsValid` _capsulecomponent_2
            (:`Is Valid`
              (set `self.playerCapsuleRadius` (`CapsuleComponent.GetScaledCapsuleRadius` _capsulecomponent_2))
              (`PrimitiveComponent.IgnoreActorWhenMoving` (`MovementComponent.UpdatedPrimitive` (`Character.CharacterMovement` _asbp_enemy)) _targetwall true)
              (`PrimitiveComponent.SetCollisionResponseToChannel` (`/Game/Blueprints/BP_wall.Cube` _targetwall) "ECC_Camera" "ECR_Ignore"))
            (:`Is Not Valid`
              (`KismetSystemLibrary.PrintString` "un able to detect capsule"))))
        (:`CastFailed`
          (bind _asbp_crate (cast `/Game/Blueprints/Button_Puzzle/BP_Crate` OtherActor))
          (`PrimitiveComponent.WakeRigidBody` (`/Game/Blueprints/Button_Puzzle/BP_Crate.StaticMesh` _asbp_crate) "None")
          (`PrimitiveComponent.SetCollisionResponseToChannel` (`/Game/Blueprints/BP_wall.Cube` (`self.TargetWall`)) "ECC_GameTraceChannel3" "ECR_Ignore"))))))

(event `self.ReceiveActorEndOverlap`
  (params (OtherActor :type "Actor Object Reference"))
  (bind _targetwall (`self.TargetWall`))
  (bind _targetwall_2 (`self.TargetWall`))
  (bind _asbp_first_person_character (cast `/Game/FirstPerson/Blueprints/BP_FirstPersonCharacter` OtherActor)
    (:`then`
      (`PrimitiveComponent.IgnoreActorWhenMoving` (`MovementComponent.UpdatedPrimitive` (`Character.CharacterMovement` _asbp_first_person_character)) _targetwall_2 false)
      (`PrimitiveComponent.SetCollisionResponseToChannel` (`/Game/Blueprints/BP_wall.Cube` _targetwall_2) "ECC_Camera" "ECR_Block"))
    (:`CastFailed`
      (bind _asbp_enemy (cast `/Game/Blueprints/Enemy/BP_Enemy` OtherActor)
        (:`then`
          (`PrimitiveComponent.IgnoreActorWhenMoving` (`MovementComponent.UpdatedPrimitive` (`Character.CharacterMovement` _asbp_enemy)) _targetwall false)
          (`PrimitiveComponent.SetCollisionResponseToChannel` (`/Game/Blueprints/BP_wall.Cube` _targetwall) "ECC_Camera" "ECR_Block"))
        (:`CastFailed`
          (cast `/Game/Blueprints/Button_Puzzle/BP_Crate` OtherActor)
          (`PrimitiveComponent.SetCollisionResponseToChannel` (`/Game/Blueprints/BP_wall.Cube` (`self.TargetWall`)) "ECC_GameTraceChannel3" "ECR_Block"))))))

(fn `TryTransfer`
  (params (OtherActor :type "Actor Object Reference") (bFrontToBack :type Boolean))
  (returns (`didTransfer?` :type Boolean))
  (bind _returnvalue (`self.GetVelocity` OtherActor))
  (bind _directionthreshold (`self.directionThreshold`))
  (bind _returnvalue_2 (`KismetMathLibrary.Dot_VectorVector` (`KismetMathLibrary.Normal` _returnvalue) (`self.HoleNormal`)))
  (bind _returnvalue_3 (* (+ (`self.ExitOffset`) (* 0.5 (`self.wallThicknessGuess`))) (`self.HoleNormal`)))
  (if (== self OtherActor)
    (`KismetSystemLibrary.PrintString` "actor is self")
    (return false)
    (elif (== OtherActor (`self.TargetWall`))
      (`KismetSystemLibrary.PrintString` "actor is target wall")
      (return false)
      (elif (< (`self.CurrentRadius`) 10.0)
        (`KismetSystemLibrary.PrintString` "hole to small")
        (return false)
        (elif (< (`KismetMathLibrary.VSize` _returnvalue) 10.0)
          (return false)
          (else
            (if bFrontToBack
              (if (< _returnvalue_2 (* _directionthreshold -1.0))
                (bind (_sweephitresult _returnvalue_4) (`self.K2_SetActorLocation` OtherActor (- (`self.HoleCenter`) _returnvalue_3) false true))
                (return _returnvalue_4)
                (else
                  _))
              (elif (> _returnvalue_2 _directionthreshold)
                (bind (_sweephitresult_2 _returnvalue_5) (`self.K2_SetActorLocation` OtherActor (+ _returnvalue_3 (`self.HoleCenter`)) false true))
                (return _returnvalue_5)
                (else
                  _)))
            (return false)))))))

(fn `UserConstructionScript`)